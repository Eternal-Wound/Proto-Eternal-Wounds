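; BP_Rope is a swingable rope actor that the player can grab.
; Its capsule checks overlapping actors with IsArmMessage and passes itself to arms through GrabRopeMessage, alongside a debug "Hello" print.
; AddSwingForce pushes the Endrope component with a scaled, mass-independent force, but only while that end hangs less than a set height below the actor's origin, which limits the swing.
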(event OnComponentBeginOverlap(Capsule)
  (params (OverlappedComponent :type Primitive%20Component%20Object%20Reference) (OtherActor :type Actor%20Object%20Reference) (OtherComp :type Primitive%20Component%20Object%20Reference) (OtherBodyIndex :type Integer) (bFromSweep :type Boolean) (SweepResult :type Hit%20Result%20Structure%20%28by%20ref%29))
  ;[1 1 1] Check et active la fonction grab rope chez le joueur
  (bind _yes_no (Class|BPIPlayer|IsArm(Message) OtherActor))
  (if _yes_no
    (Class|BPIPlayer|GrabRope(Message) OtherActor self)
    (Development|PrintText "Hello")))

(event Custom|AddSwingForce
  (params (Force :type Vector))
  (if (< (- (.z (Transformation|GetActorLocation)) (.z (Transformation|GetWorldLocation (Variables|Default|Getendrope)))) 5e+02)
    (Physics|AddForce (Variables|Default|Getendrope) (* Force 5e+02) "None" true)))

(event EventBeginPlay)

(event Collision|EventActorBeginOverlap
  (params (OtherActor :type Actor%20Object%20Reference)))

(event EventTick
  (params (DeltaSeconds :type Float%20%28single-precision%29)))

(fn ConstructionScript)